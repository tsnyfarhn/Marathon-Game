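; AI character that follows a fixed route through thirteen waypoint actors.
; After a short delay on BeginPlay, it chains AIMoveTo calls, each started by the success of the previous one.
; Walk speed switches between a faster and slower value on certain legs.
; The route runs once without looping, and no failure branch is handled, so a failed move ends it.
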(event EventBeginPlay
  ;[1 1 1] AI Path Follow
  (Utilities|FlowControl|Delay 3.0)
  (Variables|/Script/Engine.CharacterMovementComponent|SetMaxWalkSpeed (Variables|Character|GetCharacterMovement) 6e+02)
  (AI|AIMoveTo self "0, 0, 0" (Variables|Default|GetWaipoint_01) 5.0 false
    (:OnSuccess
      (AI|AIMoveTo self "0, 0, 0" (Variables|Default|GetWaipoint_02) 5.0 false
        (:OnSuccess
          (Variables|/Script/Engine.CharacterMovementComponent|SetMaxWalkSpeed (Variables|Character|GetCharacterMovement) 4e+02)
          (AI|AIMoveTo self "0, 0, 0" (Variables|Default|GetWaipoint_03) 5.0 false
            (:OnSuccess
              (Variables|/Script/Engine.CharacterMovementComponent|SetMaxWalkSpeed (Variables|Character|GetCharacterMovement) 6e+02)
              (AI|AIMoveTo self "0, 0, 0" (Variables|Default|GetWaipoint_04) 5.0 false
                (:OnSuccess
                  (AI|AIMoveTo self "0, 0, 0" (Variables|Default|GetWaipoint_05) 5.0 false
                    (:OnSuccess
                      (Variables|/Script/Engine.CharacterMovementComponent|SetMaxWalkSpeed (Variables|Character|GetCharacterMovement) 6e+02)
                      (AI|AIMoveTo self "0, 0, 0" (Variables|Default|GetWaipoint_06) 5.0 false
                        (:OnSuccess
                          (Variables|/Script/Engine.CharacterMovementComponent|SetMaxWalkSpeed (Variables|Character|GetCharacterMovement) 6e+02)
                          (AI|AIMoveTo self "0, 0, 0" (Variables|Default|GetWaipoint_07) 5.0 false
                            (:OnSuccess
                              (Variables|/Script/Engine.CharacterMovementComponent|SetMaxWalkSpeed (Variables|Character|GetCharacterMovement) 6e+02)
                              (AI|AIMoveTo self "0, 0, 0" (Variables|Default|GetWaipoint_08) 5.0 false
                                (:OnSuccess
                                  (Variables|/Script/Engine.CharacterMovementComponent|SetMaxWalkSpeed (Variables|Character|GetCharacterMovement) 4e+02)
                                  (AI|AIMoveTo self "0, 0, 0" (Variables|Default|GetWaipoint_09) 5.0 false
                                    (:OnSuccess
                                      (AI|AIMoveTo self "0, 0, 0" (Variables|Default|GetWaipoint_10) 5.0 false
                                        (:OnSuccess
                                          (Variables|/Script/Engine.CharacterMovementComponent|SetMaxWalkSpeed (Variables|Character|GetCharacterMovement) 4e+02)
                                          (AI|AIMoveTo self "0, 0, 0" (Variables|Default|GetWaipoint_11) 5.0 false
                                            (:OnSuccess
                                              (Variables|/Script/Engine.CharacterMovementComponent|SetMaxWalkSpeed (Variables|Character|GetCharacterMovement) 6e+02)
                                              (AI|AIMoveTo self "0, 0, 0" (Variables|Default|GetWaipoint_12) 5.0 false
                                                (:OnSuccess
                                                  (Variables|/Script/Engine.CharacterMovementComponent|SetMaxWalkSpeed (Variables|Character|GetCharacterMovement) 4e+02)
                                                  (AI|AIMoveTo self "0, 0, 0" (Variables|Default|GetWaipoint_13) 5.0 false))))))))))))))))))))))))))

(fn ConstructionScript)